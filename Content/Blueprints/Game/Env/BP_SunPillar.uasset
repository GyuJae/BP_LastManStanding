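; BP_SunPillar is an environment pillar that notifies the game mode when a player touches it.
; At BeginPlay it disables its capsule's collision on non-server instances, so overlap detection runs only on the server.
; When a BP_Player overlaps the capsule, it passes that player's state and itself to BP_GameMode's OnTriggerSubPillar, leaving any response to the game mode.
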(event OnComponentBeginOverlap(Capsule)
  (params (OverlappedComponent :type Primitive%20Component%20Object%20Reference) (OtherActor :type Actor%20Object%20Reference) (OtherComp :type Primitive%20Component%20Object%20Reference) (OtherBodyIndex :type Integer) (bFromSweep :type Boolean) (SweepResult :type Hit%20Result%20Structure%20%28by%20ref%29))
  ;[0.15 0.15 0.15 0.5] Sub Pillar
  (bind _asbp_player (Utilities|Casting|CastToBP_Player OtherActor))
  (bind _asbp_game_mode (Utilities|Casting|CastToBP_GameMode (Game|GetGameMode)))
  (Default|OnTriggerSubPillar _asbp_game_mode (Default|GetBPPlayerState _asbp_player) self))

(event EventBeginPlay
  (if (not (Networking|IsServer))
    (Collision|SetCollisionEnabled (Variables|Default|GetCapsule) "NoCollision")))

(fn ConstructionScript)
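; Game mode that populates the level with NPCs and ends a last-player-standing match.
; On BeginPlay it spawns BP_Npc actors at random reachable navmesh points within a wide radius of a PlayerStart.
; OnPlayerDeath flags the player state dead, then GetWinner scans the PlayerArray for a sole living BP_PlayerState.
; A valid winner sets IsGameOver and calls EndGame, which only prints a game-over message.
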(event EventBeginPlay
  (CallFunction|SpawnNpc (Variables|Default|GetNpcSpawnCount)))

(fn ConstructionScript)

(fn SpawnNpc
  (params (InNpcSpawnCount :type Integer))
  (for _index (range 0 InNpcSpawnCount)
    (bind _returnvalue (Actor|GetActorOfClass "/Script/Engine.PlayerStart"))
    (if (.ReturnValue (AI|Navigation|GetRandomReachablePointinRadius (Transformation|GetActorLocation _returnvalue) 5e+04 0 0))
      (Game|SpawnActorfromClass "/Game/Blueprints/Game/Characters/Npc/BP_Npc.BP_Npc_C" (Math|Transform|MakeTransform (.RandomLocation (AI|Navigation|GetRandomReachablePointinRadius (Transformation|GetActorLocation _returnvalue) 5e+04 0 0)) "0, 0, 0" "1.000000,1.000000,1.000000") "AdjustIfPossibleButAlwaysSpawn" "MultiplyWithRoot" 0 0))))

(fn OnPlayerDeath
  (params (InPlayerState :type BP%20Player%20State%20Object%20Reference))
  ;[0.15 0.15 0.15 0.5] On Player Death
  (Variables|/Game/Blueprints/Game/Characters/Player/BP_PlayerState.BP_PlayerState_C|SetIsDead InPlayerState true)
  (if (not (Variables|Default|GetIsGameOver))
    (Utilities|IsValid (CallFunction|GetWinner)
      (:Is%20Valid
        (Utilities|FlowControl|Sequence
          (:then_0
            (Variables|Default|SetIsGameOver true))
          (:then_1
            (CallFunction|EndGame)))))))

(fn GetWinner
  (Utilities|FlowControl|Sequence
    (:then_0
      ;[0.15 0.15 0.15 0.5] Alive Count
      (for _array_element (Variables|/Script/Engine.GameStateBase|GetPlayerArray (Game|GetGameState))
        (bind _asbp_player_state (Utilities|Casting|CastToBP_PlayerState _array_element))
        (if (not (Variables|/Game/Blueprints/Game/Characters/Player/BP_PlayerState.BP_PlayerState_C|GetIsDead _asbp_player_state))
          (Math|Integer|IncrementInt (LocalVariables|GetAliveCount)))))
    (:then_1
      ;[0.15 0.15 0.15 0.5] Get Winner (Alive)
      (if (== (LocalVariables|GetAliveCount) 1)
        (for _array_element_2 (Variables|/Script/Engine.GameStateBase|GetPlayerArray (Game|GetGameState))
          (bind _asbp_player_state_2 (Utilities|Casting|CastToBP_PlayerState _array_element_2))
          (if (not (Variables|/Game/Blueprints/Game/Characters/Player/BP_PlayerState.BP_PlayerState_C|GetIsDead _asbp_player_state_2))
            (return _asbp_player_state_2)))))
    (:then_2
      (return 0))))

(fn EndGame
  (Development|PrintString "Game Over!!!"))